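; BP_Unite is a data-driven unit Character whose construction script applies mesh, animation, capsule height and walk speed from StructUnit.
; CallPower selects a special power: a small speed boost or a repeating summon timer.
; SummonEvent spawns a half-scale BP_Unite using the Skeleton row of DT_Unit.
; Attack cycles four melee montages, buffering input for ComboAttackSave until ResetCombo clears it; damage is only printed.
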(event Custom|Attack
  ;[1 1 1] Combo System Setup.
  (Variables|Default|SetMeleeSpeed 1.0)
  (if (Variables|Default|GetIsAttacking)
    (Variables|Default|SetSaveAttack true)
    (else
      (Variables|Default|SetIsAttacking true)
      (Variables|Default|SetAttackHit? false)
      (switch int (Variables|Default|GetAttackCount)
        (:0
          (Variables|Default|SetAttackCount 1)
          (Animation|PlayAnimMontage "/Game/Characters/Heroes/Terra/Animations/Primary_Melee_A_slow_Montage.Primary_Melee_A_slow_Montage" (Variables|Default|GetMeleeSpeed) "None"))
        (:1
          (Variables|Default|SetAttackCount 2)
          (Animation|PlayAnimMontage "/Game/Characters/Heroes/Terra/Animations/Primary_Melee_B_slow_Montage.Primary_Melee_B_slow_Montage" (Variables|Default|GetMeleeSpeed) "None"))
        (:2
          (Variables|Default|SetAttackCount 3)
          (Animation|PlayAnimMontage "/Game/Characters/Heroes/Terra/Animations/Primary_Melee_C_slow_Montage.Primary_Melee_C_slow_Montage" (Variables|Default|GetMeleeSpeed) "None"))
        (:3
          (Variables|Default|SetAttackCount 0)
          (Animation|PlayAnimMontage "/Game/Characters/Heroes/Terra/Animations/Primary_Melee_D_slow_Montage.Primary_Melee_D_slow_Montage" (Variables|Default|GetMeleeSpeed) "None"))))))

(event Custom|SummonEvent
  (bind _returnvalue (Transformation|GetActorTransform))
  ;[1 1 1] WitchPower
  (bind _returnvalue_2 (Utilities|GetDataTableRow "/Game/DataTables/DT_Unit.DT_Unit" "Skeleton")
    (:then
      (Game|SpawnActorfromClass "BP_Unite_C" (Math|Transform|MakeTransform (.location _returnvalue) (.rotation _returnvalue) "0.500000,0.500000,0.500000") "AdjustIfPossibleButAlwaysSpawn" 0 _returnvalue_2 self))))

(event Custom|ResetCombo
  ;[1 1 1] Combo System Setup.
  (Variables|Default|SetAttackCount 0)
  (Variables|Default|SetSaveAttack false)
  (Variables|Default|SetIsAttacking false))

(event Custom|ComboAttackSave
  (bind _meleespeed (Variables|Default|GetMeleeSpeed))
  ;[1 1 1] Combo System Setup.
  (if (Variables|Default|GetSaveAttack)
    (Variables|Default|SetSaveAttack false)
    (Variables|Default|SetAttackHit? false)
    (switch int (Variables|Default|GetAttackCount)
      (:0
        (Variables|Default|SetAttackCount 1)
        (Animation|PlayAnimMontage "/Game/Characters/Heroes/Terra/Animations/Primary_Melee_A_slow_Montage.Primary_Melee_A_slow_Montage" _meleespeed "None"))
      (:1
        (Variables|Default|SetAttackCount 2)
        (Animation|PlayAnimMontage "/Game/Characters/Heroes/Terra/Animations/Primary_Melee_B_slow_Montage.Primary_Melee_B_slow_Montage" _meleespeed "None"))
      (:2
        (Variables|Default|SetAttackCount 3)
        (Animation|PlayAnimMontage "/Game/Characters/Heroes/Terra/Animations/Primary_Melee_C_slow_Montage.Primary_Melee_C_slow_Montage" _meleespeed "None"))
      (:3
        (Variables|Default|SetAttackCount 0)
        (Animation|PlayAnimMontage "/Game/Characters/Heroes/Terra/Animations/Primary_Melee_D_slow_Montage.Primary_Melee_D_slow_Montage" _meleespeed "None")))))

(event Game|Damage|EventAnyDamage
  (params (Damage :type Float%20%28single-precision%29) (DamageType :type Damage%20Type%20Object%20Reference) (InstigatedBy :type Controller%20Object%20Reference) (DamageCauser :type Actor%20Object%20Reference))
  (Development|PrintString (Utilities|String|ToString(Float) Damage)))

(event EventBeginPlay)

(fn ConstructionScript
  (bind _structunit (Variables|Default|GetStructUnit))
  (bind (_unitname _speed _animation _mesh _height) (Utilities|Struct|BreakS_Unit _structunit))
  (Class|SkinnedMeshComponent|SetSkeletalMesh (Variables|Character|GetMesh) _mesh true)
  (Class|SkeletalMeshComponent|SetAnimClass (Variables|Character|GetMesh) _animation)
  (Transformation|SetRelativeLocation (Variables|Character|GetMesh) (Math|Vector|MakeVector 0.0 0.0 (* _height -1.0)) false false)
  (Components|Capsule|SetCapsuleHalfHeight (Variables|Collision|GetCapsuleComponent) _height true)
  (Variables|/Script/Engine.CharacterMovementComponent|SetMaxWalkSpeed (Variables|Character|GetCharacterMovement) _speed))

(fn CallPower
  (switch Utilities|FlowControl|Switch|SwitchonSpecialPower (.SpecialPower (Utilities|Struct|BreakS_Unit (Variables|Default|GetStructUnit)))
    (:NewEnumerator0
      (CallFunction|MobilityUp))
    (:NewEnumerator4
      (CallFunction|Summon))))

(fn MobilityUp
  (bind _charactermovement (Variables|Character|GetCharacterMovement))
  (Variables|/Script/Engine.CharacterMovementComponent|SetMaxWalkSpeed _charactermovement (+ (Variables|/Script/Engine.CharacterMovementComponent|GetMaxWalkSpeed _charactermovement) 1.0)))

(fn TakeDamage)

(fn Summon
  (Development|PrintString "BeginSummon")
  (Utilities|Time|SetTimerbyEvent (EventDispatchers|CreateEvent :!event Custom|SummonEvent) 7.0 true))