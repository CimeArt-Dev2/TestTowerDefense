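; AI controller for BP_Unite units that runs the BT_IA behavior tree and feeds it a destination and a target.
; SetTarget writes the unit's BaseToAttack location to the GoToLocation blackboard key.
; While Target is empty, Tick stops montages, resets the combo and scans sight-perceived units.
; Units with a different BaseToAttack count as opponents, and a distance comparison picks one to store as Target.
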(event Custom|SetTarget
  (AI|Components|Blackboard|SetValueasVector (Variables|Default|GetBlackboard) (Utilities|String|StringToName "GoToLocation") (Transformation|GetActorLocation (Variables|/Game/Blueprints/BP_Unite.BP_Unite_C|GetBaseToAttack (.AsBP%20Unite (Utilities|Casting|CastToBP_Unite (Pawn|GetControlledPawn)))))))

(event EventBeginPlay
  (AI|RunBehaviorTree "/Game/Blueprints/AI/BT_IA.BT_IA"))

(event EventTick
  (params (DeltaSeconds :type Float%20%28single-precision%29))
  (bind _returnvalue (Pawn|GetControlledPawn))
  (bind _asbp_unite (Utilities|Casting|CastToBP_Unite _returnvalue))
  (if (== (AI|Components|Blackboard|GetValueasObject (Variables|Default|GetBlackboard) (Utilities|String|StringToName "Target")) 0)
    (Animation|StopAnimMontage _asbp_unite 0)
    (Default|ResetCombo _asbp_unite)
    (bind (_array_element _array_index) (Utilities|Array|ForEachLoopwithBreak (Class|AIPerceptionComponent|GetPerceivedActors (Variables|Default|GetAIPerception) "/Script/AIModule.AISense_Sight"))
      (:LoopBody
        (bind _asbp_unite_2 (Utilities|Casting|CastToBP_Unite _array_element))
        (if (!= (Variables|/Game/Blueprints/BP_Unite.BP_Unite_C|GetBaseToAttack _asbp_unite_2) (Variables|/Game/Blueprints/BP_Unite.BP_Unite_C|GetBaseToAttack (.AsBP%20Unite (Utilities|Casting|CastToBP_Unite (Pawn|GetControlledPawn)))))
          (Variables|Default|SetFound? true)
          (if (Variables|Default|GetFirst?)
            (Variables|Default|SetFirst? false)
            (Variables|Default|SetIndex _array_index :!label _label)
            (Variables|Default|SetMinDist (Math|Vector|Distance(Vector) (Transformation|GetActorLocation) (Transformation|GetActorLocation (Pawn|GetControlledPawn))))
            (elif (< (Math|Vector|Distance(Vector) (Transformation|GetActorLocation _array_element) (Transformation|GetActorLocation (Pawn|GetControlledPawn))) (Variables|Default|GetMinDist))
              (goto _label)))))
      (:Completed
        (if (Variables|Default|GetFound?)
          (AI|Components|Blackboard|SetValueasObject (Variables|Default|GetBlackboard) (Utilities|String|StringToName "Target") (Utilities|Array|Get(acopy) (Class|AIPerceptionComponent|GetPerceivedActors (Variables|Default|GetAIPerception) "/Script/AIModule.AISense_Sight") (Variables|Default|GetIndex)))
          (Variables|Default|SetFirst? true)
          (Variables|Default|SetFound? false))))))

(fn ConstructionScript)