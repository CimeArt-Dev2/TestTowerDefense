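; Anim notify state that detects and applies a unit's attack hit during its attack animation.
; Each tick until AttackHit is set, it sphere-traces between two named mesh sockets, with debug drawing on, for a BP_Unite or BP_Base.
; A hit deals StructUnit Attack as point damage, or full radial damage when AoeZone is positive.
; It then plays the attack sound and sets AttackHit to block repeat hits.
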(fn ReceivedNotifyTick
  (params (MeshComp :type Skeletal%20Mesh%20Component%20Object%20Reference) (Animation :type Anim%20Sequence%20Base%20Object%20Reference) (FrameDeltaTime :type Float%20%28single-precision%29))
  (bind _output_get (LocalVariables|SetUnite (.AsBP%20Unite (Utilities|Casting|CastToBP_Unite (Components|GetOwner MeshComp)))))
  (if (not (Variables|/Game/Blueprints/BP_Unite.BP_Unite_C|GetAttackHit? _output_get))
    (bind _outhit (Collision|SphereTraceForObjects MeshComp (Transformation|GetSocketLocation MeshComp (Variables|Default|GetFirstSocketName)) (Transformation|GetSocketLocation MeshComp (Variables|Default|GetSecondSocketName)) 2e+01 (Utilities|Array|MakeArray "ObjectTypeQuery3" "ObjectTypeQuery2") false 0 "ForDuration"))
    (Utilities|Casting|CastToBP_Unite (.hitactor _outhit)
      (:then
        (if (<= (.AoeZone (Utilities|Struct|BreakS_Unit (Variables|/Game/Blueprints/BP_Unite.BP_Unite_C|GetStructUnit (LocalVariables|GetUnite)))) 0.0)
          (Game|Damage|ApplyDamage (.hitactor _outhit) (.Attack (Utilities|Struct|BreakS_Unit (Variables|/Game/Blueprints/BP_Unite.BP_Unite_C|GetStructUnit (LocalVariables|GetUnite)))) 0 (LocalVariables|GetUnite))
          (else
            (Game|Damage|ApplyRadialDamage MeshComp (.Attack (Utilities|Struct|BreakS_Unit (Variables|/Game/Blueprints/BP_Unite.BP_Unite_C|GetStructUnit (LocalVariables|GetUnite)))) (.location _outhit) (.AoeZone (Utilities|Struct|BreakS_Unit (Variables|/Game/Blueprints/BP_Unite.BP_Unite_C|GetStructUnit (LocalVariables|GetUnite)))) 0 0 (LocalVariables|GetUnite) 0 true "ECC_Visibility"))))
      (:CastFailed
        (Utilities|Casting|CastToBP_Base (.hitactor _outhit))
        (if (<= (.AoeZone (Utilities|Struct|BreakS_Unit (Variables|/Game/Blueprints/BP_Unite.BP_Unite_C|GetStructUnit (LocalVariables|GetUnite)))) 0.0)
          (Game|Damage|ApplyDamage (.hitactor _outhit) (.Attack (Utilities|Struct|BreakS_Unit (Variables|/Game/Blueprints/BP_Unite.BP_Unite_C|GetStructUnit (LocalVariables|GetUnite)))) 0 (LocalVariables|GetUnite))
          (else
            (Game|Damage|ApplyRadialDamage MeshComp (.Attack (Utilities|Struct|BreakS_Unit (Variables|/Game/Blueprints/BP_Unite.BP_Unite_C|GetStructUnit (LocalVariables|GetUnite)))) (.location _outhit) (.AoeZone (Utilities|Struct|BreakS_Unit (Variables|/Game/Blueprints/BP_Unite.BP_Unite_C|GetStructUnit (LocalVariables|GetUnite)))) 0 0 (LocalVariables|GetUnite) 0 true "ECC_Visibility")))))
    (Audio|PlaySoundatLocation MeshComp (.AttackSc (Utilities|Struct|BreakS_Unit (Variables|/Game/Blueprints/BP_Unite.BP_Unite_C|GetStructUnit (LocalVariables|GetUnite)))) (Transformation|GetActorLocation (LocalVariables|GetUnite)) "0, 0, 0" 1.0 1.0 0.0 0 0 0)
    (Variables|/Game/Blueprints/BP_Unite.BP_Unite_C|SetAttackHit? (LocalVariables|GetUnite) true)
    (return false)))