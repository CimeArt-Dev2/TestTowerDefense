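; BP_Player is the player pawn for a unit-spawning game with a coin economy, moved along world axes.
; BeginPlay creates the interface widget, shows the cursor and starts a one-second timer adding Income to Coins.
; Six spell inputs look up units chosen in the GameInstance in DT_Unit, then spawn affordable ones at a TargetPoint and deduct cost.
; UpIncome spends coins to multiply income, doubling its own price each purchase.
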(event Custom|AddCoin
  (Variables|Default|SetCoins (+ (Variables|Default|GetCoins) (Variables|Default|GetIncome))))

(event EventBeginPlay
  (bind _returnvalue (Game|GetPlayerController 0))
  (bind _returnvalue_2 (UserInterface|CreateWidget "/Game/Blueprints/Widgets/WG_Interface.WG_Interface_C" _returnvalue))
  (bind _output_get (Variables|Default|SetWGRef _returnvalue_2))
  (UserInterface|Viewport|AddtoViewport _output_get 0)
  (Variables|/Script/Engine.PlayerController|SetbShowMouseCursor _returnvalue true)
  (Utilities|Time|SetTimerbyEvent (delegate Custom|AddCoin) 1.0 true))

(event Input|ActionEvents|InputActionSpell1
  (params (Key :type Key%20Structure :default "None"))
  (:Pressed
    (CallFunction|CallSpell)))

(event Input|ActionEvents|InputActionSpell6
  (params (Key :type Key%20Structure :default "None"))
  (:Pressed
    (CallFunction|CallSpell 5)))

(event Input|ActionEvents|InputActionSpell2
  (params (Key :type Key%20Structure :default "None"))
  (:Pressed
    (CallFunction|CallSpell 1)))

(event Input|ActionEvents|InputActionSpell3
  (params (Key :type Key%20Structure :default "None"))
  (:Pressed
    (CallFunction|CallSpell 2)))

(event Input|ActionEvents|InputActionSpell4
  (params (Key :type Key%20Structure :default "None"))
  (:Pressed
    (CallFunction|CallSpell 3)))

(event Input|ActionEvents|InputActionSpell5
  (params (Key :type Key%20Structure :default "None"))
  (:Pressed
    (CallFunction|CallSpell 4)))

(event Input|AxisEvents|InputAxisMoveRight
  (params (AxisValue :type Float%20%28single-precision%29))
  (Pawn|Input|AddMovementInput "0,1.000000,0.000000" (* AxisValue 5e+01) false))

(event Input|AxisEvents|InputAxisMoveUp
  (params (AxisValue :type Float%20%28single-precision%29))
  (Pawn|Input|AddMovementInput "0.000000, 0,1.000000" (* AxisValue 5e+01) false))

(event Input|AxisEvents|InputAxisMoveForward
  (params (AxisValue :type Float%20%28single-precision%29))
  (Pawn|Input|AddMovementInput "1.000000, 0,0.000000" (* AxisValue 5e+01) false))

(fn ConstructionScript)

(fn CallSpell
  (params (Spell :type Integer))
  (bind _returnvalue (Game|GetGameInstance))
  (bind _asbp_game_instance (Utilities|Casting|CastToBP_GameInstance _returnvalue))
  (bind _unitstaken (Variables|/Game/Blueprints/Core/BP_GameInstance.BP_GameInstance_C|GetUnitsTaken _asbp_game_instance))
  (bind _output (Utilities|Array|Get(acopy) _unitstaken Spell))
  (if (<= Spell (Utilities|Array|LastIndex _unitstaken))
    (bind _returnvalue_2 (Utilities|GetDataTableRow "/Game/DataTables/DT_Unit.DT_Unit" _output)
      (:then
        (if (>= (Variables|Default|GetCoins) (.cost (Utilities|Struct|BreakS_Unit _returnvalue_2)))
          (bind _returnvalue_3 (Actor|GetActorOfClass "/Script/Engine.TargetPoint"))
          (Game|SpawnActorfromClass "/Game/Blueprints/BP_Unite.BP_Unite_C" (Transformation|GetActorTransform _returnvalue_3) "Undefined" 0 _returnvalue_2 _output self)
          (Variables|Default|SetCoins (- (Variables|Default|GetCoins) (.cost (Utilities|Struct|BreakS_Unit _returnvalue_2)))))))))

(fn UpIncome
  (if (>= (Variables|Default|GetCoins) (Variables|Default|GetCostUpIncome))
    (Variables|Default|SetIncome (Math|Float|Truncate (* (Variables|Default|GetIncome) (Variables|Default|GetRatioIncome))))
    (Variables|Default|SetRatioIncome (+ (Variables|Default|GetRatioIncome) 0.0))
    (Variables|Default|SetCoins (- (Variables|Default|GetCoins) (Variables|Default|GetCostUpIncome)))
    (Variables|Default|SetCostUpIncome (* (Variables|Default|GetCostUpIncome) 2))))