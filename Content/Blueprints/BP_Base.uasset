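; BP_Base is a destructible team base that spawns units to attack the opposing base.
; On BeginPlay it finds the other base and either registers with BP_Player or, as AI, spawns a DT_Unit Paladin every few seconds.
; SpawnUnit places BP_Unite at the active spawn point, which SwitchActiveSpawnPoint cycles.
; Damage lowers health; the player base plays a throttled alert or triggers Lose at zero, while enemy base destruction is unhandled.
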(event EventBeginPlay
  (Utilities|FlowControl|Sequence
    (:then_0
      ;[1 1 1] GetEnemyBase
      (bind _outactors (Actor|GetAllActorsOfClass "BP_Base_C"))
      (bind _array_element (Utilities|Array|ForEachLoopwithBreak _outactors :!label _label)
        (:LoopBody
          (if (!= _array_element self)
            (Variables|Default|SetEnemyBase _array_element)
            (goto _label Break)))))
    (:then_1
      ;[1 1 1] IsPlayerBase?
      (if (Variables|Default|GetPlayerBase?)
        (Variables|/Game/Blueprints/BP_Player.BP_Player_C|SetBase (.AsBP%20Player (Utilities|Casting|CastToBP_Player (Game|Player|GetPlayerPawn 0))) self)))
    (:then_2
      (Development|PrintString "Hello")
      (if (not (Variables|Default|GetPlayerBase?))
        (bind _returnvalue (Utilities|GetDataTableRow "/Game/DataTables/DT_Unit.DT_Unit" "Paladin" :!label _label_2)
          (:then
            (CallFunction|SpawnUnit _returnvalue)
            (Utilities|FlowControl|Delay 4.0)
            (goto _label_2)))))))

(event Game|Damage|EventAnyDamage
  (params (Damage :type Float%20%28single-precision%29) (DamageType :type Damage%20Type%20Object%20Reference) (InstigatedBy :type Controller%20Object%20Reference) (DamageCauser :type Actor%20Object%20Reference))
  (bind _output_get (Variables|Default|SetHealth (- (Variables|Default|GetHealth) Damage)))
  (Audio|PlaySound2D "/Game/SoundDesign/Base_Sound/SC/Base_BeingHit_SC.Base_BeingHit_SC" 0.5 1.0 0.0 0 0)
  (if (Variables|Default|GetPlayerBase?)
    (if (<= _output_get 0.0)
      (if (Variables|Default|GetPlayerBase?)
        (bind _asbp_player (Utilities|Casting|CastToBP_Player (Game|Player|GetPlayerPawn 0)))
        (Default|Lose _asbp_player)
        (else
          (Development|PrintString "vous avez gagnez")))
      (else
        (Utilities|FlowControl|DoOnce false :!label _label
          (:Completed
            (Audio|PlaySound2D "/Game/SoundDesign/Base_Sound/SC/Base_Alert_SC.Base_Alert_SC" 0.75 1.0 0.0 0 0)
            (Utilities|FlowControl|Delay 1e+01)
            (goto _label Reset)))))))

(fn ConstructionScript)

(fn SpawnUnit
  (params (StructUnit :type S%20Unit%20Structure))
  (bind _spawnpoints (Variables|Default|GetSpawnPoints))
  (bind _activespawnpoint (Variables|Default|GetactiveSpawnPoint))
  (bind _output (Utilities|Array|Get(acopy) _spawnpoints _activespawnpoint))
  ;[1 1 1] Verif nul
  (if (Utilities|Name|NotEqual(Name) (.UnitName (Utilities|Struct|BreakS_Unit StructUnit)) "None")
    (Game|SpawnActorfromClass "/Game/Blueprints/BP_Unite.BP_Unite_C" (Math|Transform|MakeTransform (+ (Transformation|GetActorLocation) (.location _output)) (.rotation _output) "1,1,1") "Undefined" 0 StructUnit (Variables|Default|GetEnemyBase) self)))

(fn SwitchActiveSpawnPoint
  (if (>= (Variables|Default|GetactiveSpawnPoint) (Utilities|Array|LastIndex (Variables|Default|GetSpawnPoints)))
    (Variables|Default|SetactiveSpawnPoint 0)
    (else
      (Math|Integer|IncrementInt (Variables|Default|GetactiveSpawnPoint)))))