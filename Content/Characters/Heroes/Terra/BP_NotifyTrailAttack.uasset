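; Trail-style anim notify state for Terra that deals melee attack damage to BP_Unite units during an animation.
; Each tick until the owner's AttackHit flag is set, it sphere-traces Pawns between the two trail sockets, with debug drawing on.
; A BP_Unite hit triggers full radial damage at the impact point, ignoring the owner, then sets AttackHit to prevent repeat hits.
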(fn ReceivedNotifyTick
  (params (MeshComp :type Skeletal%20Mesh%20Component%20Object%20Reference) (Animation :type Anim%20Sequence%20Base%20Object%20Reference) (FrameDeltaTime :type Float%20%28single-precision%29))
  (bind _returnvalue (Components|GetOwner MeshComp))
  (bind _asbp_unite (Utilities|Casting|CastToBP_Unite _returnvalue))
  (if (not (Variables|/Game/Blueprints/BP_Unite.BP_Unite_C|GetAttackHit? _asbp_unite))
    (bind _outhit (Collision|SphereTraceForObjects MeshComp (Transformation|GetSocketLocation MeshComp (Variables|Default|GetFirstSocketName)) (Transformation|GetSocketLocation MeshComp (Variables|Default|GetSecondSocketName)) 2e+01 (Utilities|Array|MakeArray "ObjectTypeQuery3") false 0 "ForDuration"))
    (Utilities|Casting|CastToBP_Unite (.hitactor _outhit))
    (Game|Damage|ApplyRadialDamage MeshComp 1e+01 (.impactpoint _outhit) (Variables|Default|GetRadiusDamage) "/Script/Engine.DamageType" (Utilities|Array|MakeArray _asbp_unite) _asbp_unite 0 true "ECC_Visibility")
    (Variables|/Game/Blueprints/BP_Unite.BP_Unite_C|SetAttackHit? _asbp_unite true)
    (return false)))